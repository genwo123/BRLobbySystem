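; Player controller for the game that spawns and possesses the player's BP_Player pawn.
; On BeginPlay, the local controller passes the name and skin index stored in the lobby game instance to SpawnPlayer.
; SpawnPlayer creates the pawn at the PlayerStart returned by GetActorOfClass, giving it that name and skin plus a PlayerID concatenated from the current date and time down to milliseconds.
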(event `self.ReceiveBeginPlay`
  (bind _returnvalue (subsystem `LobbyGameInstance`))
  (if (`self.IsLocalPlayerController`)
    (`self.SpawnPlayer` (`LobbyGameInstance.PlayerName` _returnvalue) (`LobbyGameInstance.SkinIndex` _returnvalue))))

(event `SpawnPlayer`
  (params (PlayerName :type Text) (SkinIndex :type Integer))
  (bind (_returnvalue_year _returnvalue_month _returnvalue_day _returnvalue_hour _returnvalue_minute _returnvalue_second _returnvalue_millisecond) (`KismetMathLibrary.BreakDateTime` (`KismetMathLibrary.Now`)))
  (bind _returnvalue (`GameplayStatics.GetActorOfClass` "/Script/Engine.PlayerStart"))
  (bind _returnvalue_2 (`|SpawnActorFromClass` "/SimpleLobbySystem/Assets/BP_Player.BP_Player_C" (`self.GetTransform` _returnvalue) "Undefined" "OverrideRootScale" null PlayerName SkinIndex (`KismetStringLibrary.Concat_StrStr` (`KismetStringLibrary.Conv_IntToString` _returnvalue_year) (`KismetStringLibrary.Conv_IntToString` _returnvalue_month) (`KismetStringLibrary.Conv_IntToString` _returnvalue_day) (`KismetStringLibrary.Conv_IntToString` _returnvalue_hour) (`KismetStringLibrary.Conv_IntToString` _returnvalue_minute) (`KismetStringLibrary.Conv_IntToString` _returnvalue_second) (`KismetStringLibrary.Conv_IntToString` _returnvalue_millisecond)) null))
  (`self.Possess` self _returnvalue_2))

(fn `UserConstructionScript`)