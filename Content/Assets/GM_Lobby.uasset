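; Lobby game mode that keeps track of the connected lobby player controllers.
; Login adds each PC_Lobby to PcList; logout removes it and has player controller 0 refresh its player list.
; FindPcById searches PcList for the controller whose BP_Citizen pawn has a matching PlayerID, stopping at any pawn that fails the cast.
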(event `self.K2_PostLogin`
  (params (NewPlayer :type "PlayerController Object Reference"))
  (bind _aspc_lobby (cast `/SimpleLobbySystem/Assets/PC_Lobby` NewPlayer))
  (`KismetArrayLibrary.Array_AddUnique` (`self.PcList`) _aspc_lobby))

(event `self.K2_OnLogout`
  (params (ExitingController :type "Controller Object Reference"))
  (bind _aspc_lobby (cast `/SimpleLobbySystem/Assets/PC_Lobby` ExitingController))
  (`KismetArrayLibrary.Array_RemoveItem` (`self.PcList`) _aspc_lobby)
  (bind _aspc_lobby_2 (cast `/SimpleLobbySystem/Assets/PC_Lobby` (`GameplayStatics.GetPlayerController` 0)))
  (`/SimpleLobbySystem/Assets/PC_Lobby.UpdatePlayerList` _aspc_lobby_2))

(fn `FindPcById`
  (params (Id :type String))
  (returns (PC :type "/SimpleLobbySystem/Assets/PC_Lobby Object Reference"))
  (for _array_element (`self.PcList`)
    (bind _asbp_citizen (cast `/Game/BP/BP_Citizen` (`Controller.K2_GetPawn` _array_element)))
    (if (`KismetStringLibrary.EqualEqual_StrStr` (`/Game/BP/BP_Citizen.PlayerID` _asbp_citizen) (`local.Id`))
      (return _array_element))))

(fn `UserConstructionScript`)