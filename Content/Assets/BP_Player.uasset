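; BP_Player is a player character that shows a name above or on it through a widget and supports selectable, replicated skins.
; On BeginPlay it passes PlayerName to its W_PlayerName widget, then calls SetSkinIndex with the current SkinIndex.
; SetSkinIndex stores the index, and its RepNotify swaps the second mesh material slot between chest-logo, green and red mannequin materials.
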(event `self.ReceiveBeginPlay`
  (bind _asw_player_name (cast `/SimpleLobbySystem/UMG/W_PlayerName` (`WidgetComponent.GetUserWidgetObject` (`self.Widget`))))
  (`/SimpleLobbySystem/UMG/W_PlayerName.SetPlayerName` _asw_player_name (`self.PlayerName`))
  (`self.SetSkinIndex` (`self.SkinIndex`)))

(event `SetSkinIndex`
  (params (SkinIndex :type Integer))
  (set `self.SkinIndex` SkinIndex))

(fn `OnRep_SkinIndex`
  (`PrimitiveComponent.SetMaterial` (`self.Mesh`) 1 (select `int` (`self.SkinIndex`) :`0` "/SimpleLobbySystem/Assets/Mannequin/Character/Materials/M_UE4Man_ChestLogo.M_UE4Man_ChestLogo" :`1` "/SimpleLobbySystem/Assets/Mannequin/Character/Materials/M_UE4Man_Green.M_UE4Man_Green" :`2` "/SimpleLobbySystem/Assets/Mannequin/Character/Materials/M_UE4Man_Red.M_UE4Man_Red" :!type "MaterialInterface Object Reference")))

(fn `UserConstructionScript`)